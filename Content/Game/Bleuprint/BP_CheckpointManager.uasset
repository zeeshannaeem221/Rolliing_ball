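; Checkpoint manager that steps the player through a sequence of hoop actors, keeping the current one active.
; BeginPlay gathers all Hoops actors in GetAllActorsOfClass order and activates the first, redundantly once per hoop.
; Activate_NextCheckpoint deactivates the current hoop and activates the next, showing Game_UI once the index reaches the array length.
; Its bounds check lets the index step one past the last hoop; tag-reading nodes are unwired.
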(event `self.ReceiveBeginPlay`
  (bind _outactors (`GameplayStatics.GetAllActorsOfClass` "/Game/Game/Bleuprint/Hoops.Hoops_C"))
  (bind _output_get (set `self.BP_Hoops` _outactors))
  (for _ _output_get
    (`/Game/Game/Bleuprint/Hoops.Activate` (`|GetArrayItem` (`self.BP_Hoops`)))))

(event `Activate_NextCheckpoint`
  (if (< (`self.Current_Index`) (- (`KismetArrayLibrary.Array_Length` (`self.BP_Hoops`)) 0))
    (`/Game/Game/Bleuprint/Hoops.Deactivate` (`|GetArrayItem` (`self.BP_Hoops`) (`self.Current_Index`)))
    (set `self.Current_Index` (+ (`self.Current_Index`) 1))
    (`/Game/Game/Bleuprint/Hoops.Activate` (`|GetArrayItem` (`self.BP_Hoops`) (`self.Current_Index`)))
    (else
      (bind _returnvalue (`|CreateWidget` "/Game/Game/UI/Game_UI.Game_UI_C"))
      (`UserWidget.AddToViewport` _returnvalue 0))))

(fn `UserConstructionScript`)